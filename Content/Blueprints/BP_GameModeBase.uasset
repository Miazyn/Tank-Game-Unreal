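; BP_GameModeBase is a game mode Blueprint that shows the start and end screens of a match.
; GameStart creates WBP_GameStart, passes it the start delay and adds it to the viewport.
; GameOver shows WBP_GameEnd with the win or loss result on Main_Map only, and prints a "Snow Map" string on any other level.
; Two input mode calls are left unconnected and never run.
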(event `self.GameStart`
  (bind _returnvalue (`|CreateWidget` "/Game/Blueprints/UI/WBP_GameStart.WBP_GameStart_C"))
  (`/Game/Blueprints/UI/WBP_GameStart.SetStartDelay` _returnvalue (`self.StartDelay`))
  (`UserWidget.AddToViewport` _returnvalue 0))

(event `self.GameOver`
  (params (PlayerWon :type Boolean))
  (bind _returnvalue (`GameplayStatics.GetCurrentLevelName` true))
  (if (`KismetStringLibrary.EqualEqual_StrStr` _returnvalue "Main_Map")
    (bind _returnvalue_2 (`|CreateWidget` "/Game/Blueprints/UI/WBP_GameEnd.WBP_GameEnd_C"))
    (`/Game/Blueprints/UI/WBP_GameEnd.SetPlayerWon` _returnvalue_2 PlayerWon)
    (`UserWidget.AddToViewport` _returnvalue_2 0)
    (else
      (`KismetSystemLibrary.PrintString` "Snow Map"))))

(fn `UserConstructionScript`)